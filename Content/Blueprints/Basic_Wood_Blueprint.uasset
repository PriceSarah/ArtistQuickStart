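; Basic wood actor that floats up and down while slowly or quickly spinning in yaw, depending on its Speed variable.
; Each Tick adds the frame-to-frame change in the sine of time since creation to Z, so it bobs relative to its current position without storing an origin.
; Speed scales both bob amplitude and yaw rate.
; BeginPlay, overlap and construction script are empty.
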(event `self.ReceiveTick`
  (params (DeltaSeconds :type "Float (single-precision)"))
  (bind (_newlocation_x _newlocation_y _newlocation_z) (`KismetMathLibrary.BreakVector` (`self.NewLocation`)))
  (bind (_newrotation_roll _newrotation_pitch _newrotation_yaw) (`KismetMathLibrary.BreakRotator` (`self.NewRotation`)))
  (set `self.NewLocation` (`self.K2_GetActorLocation`))
  (set `self.NewRotation` (`self.K2_GetActorRotation`))
  (bind _output_get (set `self.RunningTime` (`self.GetGameTimeSinceCreation`)))
  (bind _output_get_2 (set `self.DeltaHeight` (- (`KismetMathLibrary.Sin` (+ DeltaSeconds _output_get)) (`KismetMathLibrary.Sin` (`self.RunningTime`)))))
  (set `self.NewLocation` (`KismetMathLibrary.MakeVector` _newlocation_x _newlocation_y (+ _newlocation_z (* _output_get_2 (`self.Speed`)))))
  (bind _output_get_3 (set `self.DeltaRotation` (* DeltaSeconds (`self.Speed`))))
  (set `self.NewRotation` (`KismetMathLibrary.MakeRotator` _newrotation_roll _newrotation_pitch (+ _newrotation_yaw _output_get_3)))
  (`self.K2_SetActorLocationAndRotation` (`self.NewLocation`) (`self.NewRotation`)))

(fn `UserConstructionScript`)